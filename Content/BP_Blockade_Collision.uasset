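; BP_Blockade_Collision is a one-shot trigger box that seals the doorways for the Victoria boss encounter when the Player overlaps it.
; It teleports the pre-placed BP_Boss_Blockades actors to stored fog transforms, using SetEntry to send the first to the entry and the rest to the exit.
; It then adds Victoria's health meter widget to the viewport and destroys itself.
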(event `self.Box.OnComponentBeginOverlap`
  (params (OverlappedComponent :type "PrimitiveComponent Object Reference") (OtherActor :type "Actor Object Reference") (OtherComp :type "PrimitiveComponent Object Reference") (OtherBodyIndex :type Integer) (bFromSweep :type Boolean) (SweepResult :type "HitResult Structure (by ref)"))
  (cast `/Game/Blueprints/Player` OtherActor)
  (bind _outactors (`GameplayStatics.GetAllActorsOfClass` "/Game/BP_Boss_Blockades.BP_Boss_Blockades_C"))
  (for _array_element _outactors
    ;[1 1 1] Blockades are already spawned underneath the doors, so this node moves them both to block the doorways
    (if (`self.SetEntry`)
      (`self.K2_TeleportTo` _array_element (`self.ExitFogLoc`) (`self.ExitFogRot`))
      (set `self.SetExit` true)
      (else
        (`self.K2_TeleportTo` _array_element (`self.EntryFogLoc`) (`self.EntryFogRot`))
        (set `self.SetEntry` true))))
  ;[1 1 1] This node creates Victorias health bar widget before destroying BP_Blockade_Collision
  (bind _returnvalue (`|CreateWidget` "/Game/W_VictoriaHealthMeter.W_VictoriaHealthMeter_C" (`GameplayStatics.GetPlayerController` 0)))
  (`UserWidget.AddToViewport` _returnvalue 0)
  (`self.K2_DestroyActor`))

(fn `UserConstructionScript`)