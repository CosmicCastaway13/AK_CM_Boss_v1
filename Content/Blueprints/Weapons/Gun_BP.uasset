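; Gun weapon Blueprint that fires a GunProjectile when its Fire event is called.
; Fire casts player character 0 to Player, then spawns the projectile at the mesh's Muzzle socket location and scale.
; The projectile's rotation comes from the player's MagicSpawner component rather than the muzzle, so shot direction follows that component.
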(event `Fire`
  (bind _asplayer (cast `/Game/Blueprints/Player` (`GameplayStatics.GetPlayerCharacter` 0)))
  (`|SpawnActorFromClass` "/Game/Blueprints/Weapons/GunProjectile.GunProjectile_C" (`KismetMathLibrary.MakeTransform` (.location (`SceneComponent.GetSocketTransform` (`self.Mesh`) "Muzzle" "RTS_World")) (`SceneComponent.K2_GetComponentRotation` (`/Game/Blueprints/Player.MagicSpawner` _asplayer)) (.scale (`SceneComponent.GetSocketTransform` (`self.Mesh`) "Muzzle" "RTS_World"))) "Undefined" "OverrideRootScale" null null))

(fn `UserConstructionScript`
  (`parent.UserConstructionScript`))